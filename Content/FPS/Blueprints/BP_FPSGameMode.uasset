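; BP_FPSGameMode is the game mode for the FPS game, setting up the HUD and tracking score.
; On BeginPlay it prints a debug map name, adds the reticle and game UI widgets to the viewport, and keeps a reference to the game UI.
; AddScore adds points to the running score and prints the total to screen, without updating the UI widget.
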(event EventBeginPlay
  (Development|PrintString (Variables|Default|GetDebugMapName) true true "(R=0.000000,G=0.660000,B=1.000000,A=1.000000)" 5.0)
  (bind _returnvalue (UserInterface|CreateWidget "/Game/FPS/GUI/WBP_Reticle.WBP_Reticle_C"))
  (UserInterface|Viewport|AddtoViewport _returnvalue 0)
  (bind _returnvalue_2 (UserInterface|CreateWidget "/Game/FPS/GUI/WBP_GameUI.WBP_GameUI_C"))
  (bind _output_get (Variables|Default|SetGameUI _returnvalue_2))
  (UserInterface|Viewport|AddtoViewport _returnvalue_2 0))

(fn ConstructionScript)

(fn AddScore
  (params (Points :type Integer))
  (bind _output_get (Variables|Default|SetScore (+ Points (Variables|Default|GetScore))))
  (Development|PrintString (Utilities|String|ToString(Integer) _output_get)))