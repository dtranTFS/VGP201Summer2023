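; An actor component in the FPS enemy folder that tracks an enemy's health.
; On BeginPlay it sets Health to MaxHealth.
; TakeDamage subtracts damage and clamps Health between zero and MaxHealth, and IsDead reports whether Health has reached zero.
; It raises no death event itself, so owners must query IsDead.
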(event EventBeginPlay
  (Variables|Default|SetHealth (Variables|Default|GetMaxHealth)))

(fn TakeDamage
  (params (Damage :type Float%20%28double-precision%29))
  (Variables|Default|SetHealth (Math|Float|Clamp(Float) (- (Variables|Default|GetHealth) Damage) 0.0 (Variables|Default|GetMaxHealth))))

(fn IsDead
  (return (<= (Variables|Default|GetHealth) 0.0)))