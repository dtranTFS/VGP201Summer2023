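; BP_Shotgun is a shotgun Blueprint that extends a parent gun class by overriding its ShootGun function.
; The override calls the parent logic, runs one Visibility line trace between the supplied start and end positions, then prints the hit actor's name.
; It adds no spread, pellets or damage of its own, and its event graph holds only disabled default events.
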(event EventBeginPlay
  (|CallParentFunction) ; This node is disabled and will not be called.\nDrag off pins to build functionality.
)

(event Collision|EventActorBeginOverlap
  (params (OtherActor :type Actor%20Object%20Reference))
  (|CallParentFunction OtherActor) ; This node is disabled and will not be called.\nDrag off pins to build functionality.
)

(event EventTick
  (params (DeltaSeconds :type Float%20%28single-precision%29))
  (|CallParentFunction DeltaSeconds) ; This node is disabled and will not be called.\nDrag off pins to build functionality.
)

(fn ConstructionScript
  (|CallParentFunction))

(fn ShootGun
  (params (StartIngPosition :type Vector :default "0, 0, 0") (EndPosition :type Vector :default "0, 0, 0"))
  (|CallParentFunction StartIngPosition EndPosition)
  (bind _outhit (Collision|LineTraceByChannel StartIngPosition EndPosition "TraceTypeQuery1" false 0 "None"))
  (Development|PrintString (Utilities|GetObjectName (.HitActor (Collision|BreakHitResult _outhit)))))